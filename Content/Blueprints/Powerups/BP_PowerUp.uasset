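; BP_PowerUp is a pickup that offers its PowerUp type to a 2DSideScrollerCharacter overlapping it.
; If the character accepts it, the actor hides and disables its sphere collision instead of being destroyed.
; A separate ActivateTimer event, not called within this Blueprint, starts a one-shot Cooldown timer.
; On expiry it prints a message and calls RemovePowerUp on the character with a fixed enum value.
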(event `ActivateTimer`
  (`KismetSystemLibrary.K2_SetTimerDelegate` (delegate `PowerUpCooldown`) (`self.Cooldown`)))

(event `PowerUpCooldown`
  (`KismetSystemLibrary.PrintString` "POWER UP ENDED" true true (struct :`R` 1.0 :`G` 0.030993 :`A` 1.0) 5.0)
  (`/Game/2DSideScrollerBP/Blueprints/2DSideScrollerCharacter.RemovePowerUp` (stale `self.ReceiveActorBeginOverlap` _as2dside_scroller_character) "NewEnumerator0"))

(event `self.ReceiveActorBeginOverlap`
  (params (OtherActor :type "Actor Object Reference"))
  (bind _as2dside_scroller_character (cast `/Game/2DSideScrollerBP/Blueprints/2DSideScrollerCharacter` OtherActor))
  (bind _playerhasplace (`/Game/2DSideScrollerBP/Blueprints/2DSideScrollerCharacter.SetPowerUp` _as2dside_scroller_character (`self.Power Up`)))
  (if _playerhasplace
    (`self.SetActorHiddenInGame` true)
    (`PrimitiveComponent.SetCollisionEnabled` (`self.Sphere`) "NoCollision")))

(fn `UserConstructionScript`)