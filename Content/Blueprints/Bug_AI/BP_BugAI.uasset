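; Flying bug enemy for a 2D side-scroller that destroys level ground with a player-killing laser.
; StartGame either runs it along MovePoints, zapping the ground at each, or, on level "Unknown", teleports it to a WaitPoint.
; After each point it randomly continues or teleports to an unpassed point, signals the floor below to drop, and idles until the player nears or passes.
; Tick rubber-bands fly speed against the player's X position and animates the beam.
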(event `self.ReceiveBeginPlay`
  (`CharacterMovementComponent.SetMovementMode` (`self.CharacterMovement`) "MOVE_Flying" 0))

(event `/Game/Blueprints/Interfaces/BPI_GameInterface.StartGame`
  (bind _returnvalue (`GameplayStatics.GetCurrentLevelName` true))
  (if (`KismetStringLibrary.NotEqual_StrStr` _returnvalue "Unknown")
    (`self.MoveToNextLocation`)
    (else
      (`self.Teleport To Next Wait Location`))))

(event `MoveToNextLocation`
  (`AITask_MoveTo.AIMoveTo` (`AIBlueprintHelperLibrary.GetAIController` self) (0.0 0.0 0.0) (`|GetArrayItem` (`self.MovePoints`) (`self.MovePointIndex`)) -1.0 "Default" "Default" false
    (:`then`
      (goto _label :!via `Reset`))
    (:`OnMoveFinished`
      (`/Engine/EditorBlueprintResources/StandardMacros.DoOnce` false :!label _label
        (:`Completed`
          (`self.DestroyGroundBelow`)
          (`|ExecutionSequence`
            (:`then_0`
              (`/Engine/EditorBlueprintResources/StandardMacros.IncrementInt` (`self.MovePointIndex`)
                (:`  `
                  (`self.PlanNextDecision`))))))))))

(event `PlanNextDecision`
  (if (< (`KismetMathLibrary.RandomIntegerInRange` 0 3) 3)
    (`self.MoveToNextLocation`)
    (else
      (`KismetSystemLibrary.Delay` 0.5)
      (if (not (`/Game/Blueprints/Bug_AI/BP_BugMovePoints.PassedByPlayer?` (`|GetArrayItem` (`self.MovePoints`) (`self.MovePointIndex`))))
        (`self.TeleportToLocation`)
        (else
          (`/Engine/EditorBlueprintResources/StandardMacros.IncrementInt` (`self.MovePointIndex`)
            (:`  `
              (`self.PlanNextDecision`))))))))

(event `self.ReceiveTick`
  (params (DeltaSeconds :type "Float (single-precision)"))
  (`self.AdjustSpeed`)
  (if (`self.GlitchBallActive?`)
    (`SceneComponent.K2_AddRelativeLocation` (`self.LaserBeam`) (* (* (`self.GetActorUpVector`) -1.0) (* (`GameplayStatics.GetWorldDeltaSeconds`) 5000.0)) false false)))

(event `self.LaserBeamHitBox.OnComponentBeginOverlap`
  (params (OverlappedComponent :type "PrimitiveComponent Object Reference") (OtherActor :type "Actor Object Reference") (OtherComp :type "PrimitiveComponent Object Reference") (OtherBodyIndex :type Integer) (bFromSweep :type Boolean) (SweepResult :type "HitResult Structure (by ref)"))
  (bind _as2dside_scroller_character (cast `/Game/2DSideScrollerBP/Blueprints/2DSideScrollerCharacter` OtherActor))
  (`/Game/2DSideScrollerBP/Blueprints/2DSideScrollerCharacter.OnPlayerDead` _as2dside_scroller_character false))

(fn `ActivateLaserBeam`
  (bind _laserbeam (`self.LaserBeam`))
  (set `self.GlitchBallActive?` true)
  (`PaperFlipbookComponent.SetNewTime` _laserbeam 0.0)
  (`SceneComponent.SetVisibility` _laserbeam true false)
  (`ActorComponent.SetComponentTickEnabled` _laserbeam true)
  (`PrimitiveComponent.SetCollisionEnabled` (`self.LaserBeamHitBox`) "QueryOnly")
  (`KismetSystemLibrary.K2_SetTimer` null "DeactivateLaserBeam" 0.15))

(fn `AdjustSpeed`
  (bind _charactermovement (`self.CharacterMovement`))
  (bind _x (.x (`self.K2_GetActorLocation`)))
  (bind _x_2 (.x (`self.K2_GetActorLocation` (`GameplayStatics.GetPlayerCharacter` 0))))
  (if (select `bool` (`self.CheckRightSide?`) :`false` (< _x _x_2) :`true` (> _x _x_2))
    (set `CharacterMovementComponent.MaxFlySpeed` 500.0 (`self.CharacterMovement`))
    (elif (> (`KismetMathLibrary.Abs` (- _x _x_2)) 800.0)
      (set `CharacterMovementComponent.MaxFlySpeed` 700.0 _charactermovement)
      (else
        (set `CharacterMovementComponent.MaxFlySpeed` 550.0 _charactermovement)))))

(fn `CheckDistanceFromPlayer`
  (if (or (< (`KismetMathLibrary.Abs` (- (.x (`self.K2_GetActorLocation`)) (.x (`self.K2_GetActorLocation` (`GameplayStatics.GetPlayerCharacter` 0))))) 200.0) (`/Game/Blueprints/Bug_AI/BP_BugMovePoints.PassedByPlayer?` (`|GetArrayItem` (`self.MovePoints`) (`self.MovePointIndex`))))
    (`KismetSystemLibrary.K2_ClearAndInvalidateTimerHandle` (`self.DistanceCheckTimer`))
    (`KismetSystemLibrary.K2_SetTimer` null "ResumeMoving" 1.0)))

(fn `ChooseRandomHack`
  (message `/Game/Blueprints/Interfaces/BPI_Hacks.PlayerFlipCam` (`GameplayStatics.GetPlayerCharacter` 0)))

(fn `DeactivateLaserBeam`
  (bind _laserbeam (`self.LaserBeam`))
  (set `self.GlitchBallActive?` false)
  (`PrimitiveComponent.SetCollisionEnabled` (`self.LaserBeamHitBox`) "NoCollision")
  (`SceneComponent.SetVisibility` _laserbeam false false)
  (`ActorComponent.SetComponentTickEnabled` _laserbeam false)
  (`SceneComponent.K2_SetRelativeLocation` (`self.LaserBeam`) (0.0 0.0 0.0) false false))

(fn `DestroyGroundBelow`
  (bind (_anyhit_ _outhit) (`self.TraceBelow` (`self.K2_GetActorLocation`)))
  (bind (_bblockinghit _binitialoverlap _time _distance _location _impactpoint _normal _impactnormal _physmat _hitactor) (`GameplayStatics.BreakHitResult` _outhit))
  (bind (_anyhit__2 _outhit_2) (`self.TraceBelow` _impactpoint))
  (if _anyhit_
    (`self.ActivateLaserBeam`)
    (`GameplayStatics.PlaySound2D` "/Game/SFX/BFXR/SC_Laser.SC_Laser" 1.0 1.0 0.0 null null)
    (`GameplayStatics.PlayWorldCameraShake` "/Game/Blueprints/Environment/CamShake_LaserBeam.CamShake_LaserBeam_C" _impactpoint 0.0 10000.0)
    (`self.K2_DestroyActor` _hitactor)
    (if _anyhit__2
      (`self.K2_DestroyActor` (`.HitActor` (`GameplayStatics.BreakHitResult` _outhit_2))))))

(fn `Find Next Ground`
  (bind _returnvalue (+ (`self.K2_GetActorLocation`) (* (`self.GetActorForwardVector`) (`self.LineDistance`))))
  (bind (_outhit _returnvalue_2) (`KismetSystemLibrary.LineTraceSingle` :`Start` _returnvalue :`End` (+ _returnvalue (* (* (`self.GetActorUpVector`) -1.0) 10000.0)) :`TraceChannel` "TraceTypeQuery1" :`DrawDebugType` "Persistent"))
  (if (not _returnvalue_2)
    (set `self.LineDistance` (+ (`self.LineDistance`) 100.0))))

(fn `ResumeMoving`
  (`self.PlanNextDecision`)
  (`PaperFlipbookComponent.SetFlipbook` (`self.Sprite`) "/Game/Sprites/Bug/Fly/FB_Bug_Fly.FB_Bug_Fly"))

(fn `Teleport To Next Wait Location`
  (bind _output (`|GetArrayItem` (`self.WaitPoints`) (`self.WaitPointIndex`)))
  (set `/Game/Blueprints/Bug_AI/BP_BugWaitPoints.BugRef` self _output)
  (`self.K2_SetActorLocation` (`self.K2_GetActorLocation` _output))
  (`/Engine/EditorBlueprintResources/StandardMacros.IncrementInt` (`self.WaitPointIndex`)))

(fn `TeleportToLocation`
  (bind (_anyhit_ _outhit) (`self.TraceBelow` (`self.K2_GetActorLocation`)))
  (bind (_anyhit__2 _outhit_2) (`self.TraceBelow` (`self.K2_GetActorLocation`)))
  (`self.K2_SetActorLocation` (`self.K2_GetActorLocation` (`|GetArrayItem` (`self.MovePoints`) (`self.MovePointIndex`))))
  (`/Engine/EditorBlueprintResources/StandardMacros.IncrementInt` (`self.MovePointIndex`)
    (:`  `
      (`PaperFlipbookComponent.SetFlipbook` (`self.Sprite`) "/Game/Sprites/Bug/Idle/FB_BugIdle.FB_BugIdle")
      (bind _returnvalue (`KismetSystemLibrary.K2_SetTimer` null "CheckDistanceFromPlayer" 0.1 true))
      (set `self.DistanceCheckTimer` _returnvalue)
      (if _anyhit__2
        (message `/Game/Blueprints/Interfaces/BPI_BugsInterface.DropFloor` (`.HitActor` (`GameplayStatics.BreakHitResult` _outhit_2)))
        (if _anyhit_
          (message `/Game/Blueprints/Interfaces/BPI_BugsInterface.DropFloor` (`.HitActor` (`GameplayStatics.BreakHitResult` _outhit))))))))

(fn `TraceBelow`
  (params (Start :type "Vector Structure"))
  (returns (`AnyHit?` :type Boolean) (OutHit :type "HitResult Structure"))
  (bind (_outhit _returnvalue) (`KismetSystemLibrary.LineTraceSingle` Start (+ Start (* (* (`self.GetActorUpVector`) -1.0) 10000.0)) "TraceTypeQuery1"))
  (return _returnvalue _outhit))

(fn `UserConstructionScript`)