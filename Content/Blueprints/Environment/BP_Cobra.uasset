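; Paper2D cobra enemy that patrols between two points and bites the player.
; AIMoveTo alternates patrol targets with a wait between them, until the Vision overlap halts movement and starts the attack flipbook.
; Tick keys off flipbook frames and player overlap to lunge, enable DamageCollision and play the bite sound, or resume patrol, gated by DoOnce nodes.
; DamageCollision overlap kills the player; a line-trace kill in DealDamage is unconnected.
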(event `self.ReceiveBeginPlay`
  (`self.GoToPoint1`))

(event `GoToPoint1`
  (bind (_returnvalue_roll _returnvalue_pitch) (`KismetMathLibrary.BreakRotator` (`self.K2_GetActorRotation`)))
  (bind (_returnvalue_roll_2 _returnvalue_pitch_2 _returnvalue_yaw) (`KismetMathLibrary.BreakRotator` (`KismetMathLibrary.FindLookAtRotation` (`SceneComponent.K2_GetComponentLocation` (`self.PaperFlipbook`)) (`self.K2_GetActorLocation` (`self.PatrolPoint1`)))))
  (if (!= (`self.Attack?`) true)
    (`|AIMoveTo` self (0.0 0.0 0.0) (`self.PatrolPoint1`)
      (:`then`
        (`self.K2_SetActorRotation` (`KismetMathLibrary.MakeRotator` _returnvalue_roll _returnvalue_pitch (+ _returnvalue_yaw 180.0))))
      (:`OnSuccess`
        (set `self.Patrol1?` false)
        (set `self.Patrol2?` true)
        (if (!= (`self.Attack?`) true)
          (`KismetSystemLibrary.Delay` (`self.PatrolWaitDelay`))
          (`self.GoToPoint2`))))))

(event `GoToPoint2`
  (bind (_returnvalue_roll _returnvalue_pitch) (`KismetMathLibrary.BreakRotator` (`self.K2_GetActorRotation`)))
  (bind (_returnvalue_roll_2 _returnvalue_pitch_2 _returnvalue_yaw) (`KismetMathLibrary.BreakRotator` (`KismetMathLibrary.FindLookAtRotation` (`SceneComponent.K2_GetComponentLocation` (`self.PaperFlipbook`)) (`self.K2_GetActorLocation` (`self.PatrolPoint2`)))))
  (if (!= (`self.Attack?`) true)
    (`|AIMoveTo` self (0.0 0.0 0.0) (`self.PatrolPoint2`)
      (:`then`
        (`self.K2_SetActorRotation` (`KismetMathLibrary.MakeRotator` _returnvalue_roll _returnvalue_pitch (+ _returnvalue_yaw 180.0))))
      (:`OnSuccess`
        (set `self.Patrol1?` true)
        (set `self.Patrol2?` false)
        (if (!= (`self.Attack?`) true)
          (`KismetSystemLibrary.Delay` (`self.PatrolWaitDelay`))
          (`self.GoToPoint1`))))))

(event `self.ReceiveTick`
  (params (DeltaSeconds :type "Float (single-precision)"))
  (bind _paperflipbook (`self.PaperFlipbook`))
  (bind _paperflipbook_2 (`self.PaperFlipbook`))
  (bind _paperflipbook_3 (`self.PaperFlipbook`))
  (if (== (`PaperFlipbookComponent.GetFlipbook` (`self.PaperFlipbook`)) "/Game/Sprites/Cobra/Attack/FB_Cobra_Attack.FB_Cobra_Attack")
    (if (`self.IsOverlappingActor` (`GameplayStatics.GetPlayerCharacter` 0))
      (if (== (`PaperFlipbookComponent.GetPlaybackPositionInFrames` (`self.PaperFlipbook`)) 3)
        (`self.LaunchForward`)
        (`/Engine/EditorBlueprintResources/StandardMacros.DoOnce` false :!label _label
          (:`Completed`
            (`self.DealDamage`)
            (goto _label_3 :!via `Reset`)))
        (else
          (`|ExecutionSequence`
            (:`then_0`
              (if (== (`PaperFlipbookComponent.GetPlaybackPositionInFrames` (`self.PaperFlipbook`)) 4)
                (if (not (`self.IsOverlappingActor` (`GameplayStatics.GetPlayerCharacter` 0)))
                  (`/Engine/EditorBlueprintResources/StandardMacros.DoOnce` false :!label _label_2
                    (:`Completed`
                      ;[1 1 1] Stop attack anim
                      (`PaperFlipbookComponent.Stop` _paperflipbook_2)
                      (`KismetSystemLibrary.Delay` 0.2)
                      (`PaperFlipbookComponent.SetFlipbook` _paperflipbook_2 "/Game/Sprites/Cobra/FB_Cobra.FB_Cobra")
                      (`PaperFlipbookComponent.PlayFromStart` _paperflipbook_2)
                      (if (`self.Patrol1?`)
                        (`self.GoToPoint1`)
                        (else
                          (`self.GoToPoint2`)))))
                  (else
                    (`/Engine/EditorBlueprintResources/StandardMacros.DoOnce` false :!label _label_3
                      (:`Completed`
                        (`PaperFlipbookComponent.Stop` _paperflipbook)
                        (`KismetSystemLibrary.Delay` 0.2)
                        (`PaperFlipbookComponent.SetFlipbook` _paperflipbook "/Game/Sprites/Cobra/FB_Cobra.FB_Cobra")
                        (`KismetSystemLibrary.Delay` (`self.AttackDelay`))
                        (`PaperFlipbookComponent.SetFlipbook` _paperflipbook_3 "/Game/Sprites/Cobra/Attack/FB_Cobra_Attack.FB_Cobra_Attack")
                        (`PaperFlipbookComponent.PlayFromStart` _paperflipbook_3)))))))
            (:`then_1`
              (goto _label :!via `Reset`)))))
      (else
        (goto _label_2)))))

(event `self.Vision.OnComponentBeginOverlap`
  (params (OverlappedComponent :type "PrimitiveComponent Object Reference") (OtherActor :type "Actor Object Reference") (OtherComp :type "PrimitiveComponent Object Reference") (OtherBodyIndex :type Integer) (bFromSweep :type Boolean) (SweepResult :type "HitResult Structure (by ref)"))
  (if (`self.ActorHasTag` OtherActor "Player")
    (`/Engine/EditorBlueprintResources/StandardMacros.DoOnce` false :!label _label_4
      (:`Completed`
        (set `self.Attack?` true)
        (`MovementComponent.StopMovementImmediately` (`self.FloatingPawnMovement`))
        (`PaperFlipbookComponent.SetFlipbook` (`self.PaperFlipbook`) "/Game/Sprites/Cobra/Attack/FB_Cobra_Attack.FB_Cobra_Attack")
        (goto _label_2 :!via `Reset`)))))

(event `self.Vision.OnComponentEndOverlap`
  (params (OverlappedComponent :type "PrimitiveComponent Object Reference") (OtherActor :type "Actor Object Reference") (OtherComp :type "PrimitiveComponent Object Reference") (OtherBodyIndex :type Integer))
  (if (`self.ActorHasTag` OtherActor "Player")
    (`|ExecutionSequence`
      (:`then_0`
        (set `self.Attack?` false)
        (`PrimitiveComponent.SetCollisionEnabled` (`self.DamageCollision`) "NoCollision"))
      (:`then_1`
        (goto _label_4 :!via `Reset`)))))

(event `self.DamageCollision.OnComponentBeginOverlap`
  (params (OverlappedComponent :type "PrimitiveComponent Object Reference") (OtherActor :type "Actor Object Reference") (OtherComp :type "PrimitiveComponent Object Reference") (OtherBodyIndex :type Integer) (bFromSweep :type Boolean) (SweepResult :type "HitResult Structure (by ref)"))
  (bind _as2dside_scroller_character (cast `/Game/2DSideScrollerBP/Blueprints/2DSideScrollerCharacter` OtherActor))
  (`/Engine/EditorBlueprintResources/StandardMacros.DoOnce` false :!label _label_5
    (:`Completed`
      (`/Game/2DSideScrollerBP/Blueprints/2DSideScrollerCharacter.OnPlayerDead` _as2dside_scroller_character true))))

(event `self.DamageCollision.OnComponentEndOverlap`
  (params (OverlappedComponent :type "PrimitiveComponent Object Reference") (OtherActor :type "Actor Object Reference") (OtherComp :type "PrimitiveComponent Object Reference") (OtherBodyIndex :type Integer))
  (if (`self.ActorHasTag` OtherActor "Player")
    (goto _label_5 :!via `Reset`)))

(fn `DealDamage`
  (`PrimitiveComponent.SetCollisionEnabled` (`self.DamageCollision`) "QueryOnly")
  (`GameplayStatics.PlaySound2D` "/Game/SFX/Environment/SC_SnakeBite.SC_SnakeBite" 1.0 1.0 0.0 null null))

(fn `LaunchForward`
  (`self.K2_AddActorWorldOffset` (* (* (* (`KismetMathLibrary.GetForwardVector` (`SceneComponent.K2_GetComponentRotation` (`self.PaperFlipbook`))) -1.0) (`GameplayStatics.GetWorldDeltaSeconds`)) 1500.0)))

(fn `UserConstructionScript`)