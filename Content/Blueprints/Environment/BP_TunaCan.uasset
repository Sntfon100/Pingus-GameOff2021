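; BP_TunaCan is a collectible pickup that bobs vertically and awards a point when a player touches it.
; On BeginPlay it stores its starting height and drives a timeline, scaled by a speed multiplier, that lerps Z up to a maximum height offset.
; Hitbox overlaps with actors implementing BPI_PlayerInterface send AddPointMessage, play a pickup sound and destroy the can.
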(event `self.ReceiveBeginPlay`
  (bind (_returnvalue_x _returnvalue_y _returnvalue_z) (`KismetMathLibrary.BreakVector` (`self.K2_GetActorLocation`)))
  (bind (_returnvalue_x_2 _returnvalue_y_2) (`KismetMathLibrary.BreakVector` (`self.K2_GetActorLocation`)))
  (set `self.OriginalZ` _returnvalue_z)
  (`TimelineComponent.SetPlayRate` (`self.UpDownTimeline`) (`self.TimelineSpeedMultiplier`))
  (bind (_direction _alpha) (`Timeline|UpDownTimeline`)
    (:`Update`
      (`self.K2_SetActorLocation` (`KismetMathLibrary.MakeVector` _returnvalue_x_2 _returnvalue_y_2 (`KismetMathLibrary.Lerp` (`self.OriginalZ`) (+ (`self.OriginalZ`) (`self.MaxHeight`)) _alpha))))))

(event `self.Hitbox.OnComponentBeginOverlap`
  (params (OverlappedComponent :type "PrimitiveComponent Object Reference") (OtherActor :type "Actor Object Reference") (OtherComp :type "PrimitiveComponent Object Reference") (OtherBodyIndex :type Integer) (bFromSweep :type Boolean) (SweepResult :type "HitResult Structure (by ref)"))
  (if (`KismetSystemLibrary.DoesImplementInterface` OtherActor "/Game/Blueprints/Interfaces/BPI_PlayerInterface.BPI_PlayerInterface_C")
    (message `/Game/Blueprints/Interfaces/BPI_PlayerInterface.AddPoint` OtherActor)
    (`GameplayStatics.PlaySound2D` "/Game/SFX/BFXR/SC_TunaPickup.SC_TunaPickup" 1.0 1.0 0.0 null null)
    (`self.K2_DestroyActor`)))

(fn `UserConstructionScript`)