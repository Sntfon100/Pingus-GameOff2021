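; BP_Oil is an environmental oil hazard that slows the 2D side-scroller player character while it overlaps the trigger.
; On begin overlap it caches the character's MaxWalkSpeed and replaces it with SlowSpeed.
; On end overlap it restores the cached speed, which is stored in a single variable on the actor.
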(event `self.Trigger.OnComponentBeginOverlap`
  (params (OverlappedComponent :type "PrimitiveComponent Object Reference") (OtherActor :type "Actor Object Reference") (OtherComp :type "PrimitiveComponent Object Reference") (OtherBodyIndex :type Integer) (bFromSweep :type Boolean) (SweepResult :type "HitResult Structure (by ref)"))
  (bind _as2dside_scroller_character (cast `/Game/2DSideScrollerBP/Blueprints/2DSideScrollerCharacter` OtherActor))
  (bind _charactermovement (`Character.CharacterMovement` _as2dside_scroller_character))
  (set `self.PlayerOriginalMaxSpeed` (`CharacterMovementComponent.MaxWalkSpeed` _charactermovement))
  (set `CharacterMovementComponent.MaxWalkSpeed` (`self.SlowSpeed`) _charactermovement))

(event `self.Trigger.OnComponentEndOverlap`
  (params (OverlappedComponent :type "PrimitiveComponent Object Reference") (OtherActor :type "Actor Object Reference") (OtherComp :type "PrimitiveComponent Object Reference") (OtherBodyIndex :type Integer))
  (bind _as2dside_scroller_character (cast `/Game/2DSideScrollerBP/Blueprints/2DSideScrollerCharacter` OtherActor))
  (set `CharacterMovementComponent.MaxWalkSpeed` (`self.PlayerOriginalMaxSpeed`) (`Character.CharacterMovement` _as2dside_scroller_character)))

(fn `UserConstructionScript`)