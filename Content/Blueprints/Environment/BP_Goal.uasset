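; Level goal for the 2D side-scroller that disables player input when the character overlaps its Box.
; It then opens the end-level widget with its FriendName, switches to UI-only mouse input and plays a special sound for the friend "Dingus".
; In a level named "Unknown", it shows a text box instead.
; The construction script toggles between static sprite and flipbook visuals via UseFlipBook.
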(event `self.Box.OnComponentBeginOverlap`
  (params (OverlappedComponent :type "PrimitiveComponent Object Reference") (OtherActor :type "Actor Object Reference") (OtherComp :type "PrimitiveComponent Object Reference") (OtherBodyIndex :type Integer) (bFromSweep :type Boolean) (SweepResult :type "HitResult Structure (by ref)"))
  (bind _returnvalue (`GameplayStatics.GetPlayerController` 0))
  (bind _friend_name (`self.Friend Name`))
  (bind _as2dside_scroller_character (cast `/Game/2DSideScrollerBP/Blueprints/2DSideScrollerCharacter` OtherActor))
  (`self.DisableInput` _as2dside_scroller_character _returnvalue)
  (bind _returnvalue_2 (`GameplayStatics.GetCurrentLevelName` true))
  (if (`KismetStringLibrary.NotEqual_StrStr` _returnvalue_2 "Unknown")
    (bind _returnvalue_3 (`|CreateWidget` "/Game/Widgets/WB_EndLevel.WB_EndLevel_C" null _friend_name))
    (`UserWidget.AddToViewport` _returnvalue_3 0)
    (`WidgetBlueprintLibrary.SetInputMode_UIOnlyEx` _returnvalue _returnvalue_3)
    (set `PlayerController.bShowMouseCursor` true _returnvalue)
    (if (`KismetTextLibrary.EqualEqual_TextText` _friend_name "Dingus")
      (`GameplayStatics.PlaySound2D` "/Game/Sprites/Dingus/Dingus4.Dingus4" 1.0 1.0 0.0 null null))
    (else
      (bind _returnvalue_4 (`|CreateWidget` "/Game/Widgets/WB_TextBox.WB_TextBox_C" null 9 null))
      (`/Game/Widgets/WB_TextBox.UpdateText` _returnvalue_4)
      (`UserWidget.AddToViewport` _returnvalue_4 0))))

(fn `UserConstructionScript`
  (if (`self.UseFlipBook?`)
    (`SceneComponent.SetVisibility` (`self.PaperSprite`) false false)
    (`SceneComponent.SetVisibility` (`self.PaperFlipbook`) true false)
    (else
      (`SceneComponent.SetVisibility` (`self.PaperSprite`) true false)
      (`SceneComponent.SetVisibility` (`self.PaperFlipbook`) false false))))