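; BP_FlyingPlatform is an environment platform that moves up and down continuously from its placed height.
; On BeginPlay it stores its starting Z, applies SpeedMultiplier as the timeline play rate and starts rising.
; PlatformMoveTimeline lerps Z between the original height and that height plus MaxHeight, leaving X and Y unchanged.
; When the timeline finishes, the MoveUp flag selects playing or reversing it, creating an endless ping-pong.
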(event `self.ReceiveBeginPlay`
  (bind (_returnvalue_x _returnvalue_y _returnvalue_z) (`KismetMathLibrary.BreakVector` (`self.K2_GetActorLocation`)))
  (set `self.OriginalHeight` _returnvalue_z)
  (`TimelineComponent.SetPlayRate` (`self.PlatformMoveTimeline`) (`self.SpeedMultiplier`))
  (`self.MoveUp`))

(event `MoveUp`
  (bind (_returnvalue_x _returnvalue_y) (`KismetMathLibrary.BreakVector` (`self.K2_GetActorLocation`)))
  (bind _originalheight (`self.OriginalHeight`))
  (set `self.MoveUp?` true)
  (bind (_direction _alpha) (`Timeline|PlatformMoveTimeline` :!label _label)
    (:`Update`
      (`self.K2_SetActorLocation` (`KismetMathLibrary.MakeVector` _returnvalue_x _returnvalue_y (`KismetMathLibrary.Lerp` _originalheight (+ _originalheight (`self.MaxHeight`)) _alpha))))
    (:`Finished`
      (if (`self.MoveUp?`)
        (`self.MoveDown`)
        (else
          (`self.MoveUp`))))))

(event `MoveDown`
  (set `self.MoveUp?` false)
  (goto _label :!via `Reverse`))

(fn `UserConstructionScript`)