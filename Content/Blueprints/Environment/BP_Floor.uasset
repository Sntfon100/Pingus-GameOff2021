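; BP_Floor is a 2D Paper floor piece, shown as a sprite or flipbook, that can shake and fall away.
; DropFloor starts a random pitch and yaw jitter, applied through a Delay in Tick, and makes the sprite ignore the Visibility channel.
; Player overlap with the trigger waits DropDelay, then, if shaking, moves the actor steadily downward.
; The construction script configures visual, collision and trigger size.
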(event `self.ReceiveBeginPlay`
  (bind (_returnvalue_roll _returnvalue_pitch _returnvalue_yaw) (`KismetMathLibrary.BreakRotator` (`self.K2_GetActorRotation`)))
  (set `self.OriginalPitch` _returnvalue_pitch)
  (set `self.OriginalYaw` _returnvalue_yaw))

(event `self.ReceiveTick`
  (params (DeltaSeconds :type "Float (single-precision)"))
  (bind _returnvalue_roll (`KismetMathLibrary.BreakRotator` (`SceneComponent.K2_GetComponentRotation` (select `bool` (`self.isFlipBook?`) :`false` (`self.PaperSprite`) :`true` (`self.PaperFlipbook`) :!type "SceneComponent Object Reference"))))
  (if (`self.Shake?`)
    (if (not (`self.FallDown?`))
      ;[1 1 1] Shake
      (`KismetSystemLibrary.Delay` 0.1)
      (`SceneComponent.K2_SetWorldRotation` (select `bool` (`self.isFlipBook?`) :`false` (`self.PaperSprite`) :`true` (`self.PaperFlipbook`) :!type "SceneComponent Object Reference") (`KismetMathLibrary.MakeRotator` _returnvalue_roll (+ (`self.OriginalPitch`) (`KismetMathLibrary.Conv_IntToDouble` (`KismetMathLibrary.RandomIntegerInRange` -5 5))) (+ (`self.OriginalYaw`) (`KismetMathLibrary.Conv_IntToDouble` (`KismetMathLibrary.RandomIntegerInRange` -5 5)))) false false)
      (else
        (`self.K2_AddActorWorldOffset` (`KismetMathLibrary.MakeVector` 0.0 0.0 (* (* (`GameplayStatics.GetWorldDeltaSeconds`) 300.0) -1.0)))))))

(event `/Game/Blueprints/Interfaces/BPI_BugsInterface.DropFloor`
  (`PrimitiveComponent.SetCollisionResponseToChannel` (`self.PaperSprite`) "ECC_Visibility" "ECR_Ignore")
  (set `self.Shake?` true))

(event `self.Trigger.OnComponentBeginOverlap`
  (params (OverlappedComponent :type "PrimitiveComponent Object Reference") (OtherActor :type "Actor Object Reference") (OtherComp :type "PrimitiveComponent Object Reference") (OtherBodyIndex :type Integer) (bFromSweep :type Boolean) (SweepResult :type "HitResult Structure (by ref)"))
  (if (== OtherActor (`GameplayStatics.GetPlayerCharacter` 0))
    (`KismetSystemLibrary.Delay` (`self.DropDelay`))
    (if (`self.Shake?`)
      (set `self.FallDown?` true))))

(fn `UserConstructionScript`
  (`PrimitiveComponent.SetCollisionEnabled` (`self.FloorCollision`) (select `bool` (`self.FloorCollisionEnabled?`) :`false` "NoCollision" :`true` "QueryOnly" :!type "ECollisionEnabled Enum"))
  (`BoxComponent.SetBoxExtent` (`self.Trigger`) (`self.BoxExtent`) true)
  (if (`self.isFlipBook?`)
    (`PaperFlipbookComponent.SetFlipbook` (`self.PaperFlipbook`) (`self.New Flipbook`))
    (`PrimitiveComponent.SetCollisionEnabled` (`self.PaperSprite`) "NoCollision")
    (else
      (`PaperSpriteComponent.SetSprite` (`self.PaperSprite`) (`self.Sprite`))
      (`PrimitiveComponent.SetCollisionEnabled` (`self.PaperFlipbook`) "NoCollision"))))