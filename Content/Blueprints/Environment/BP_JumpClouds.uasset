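; A bouncy cloud platform that launches the 2D side-scroller character upward when it overlaps the hitbox.
; The launch overrides Z velocity using the cloud's up vector, adds a small positive X push and plays a sound.
; The sprite starts with a happy face and switches to a sad one after the first bounce.
; A timeline, started after a short random delay to desync clouds, nudges the sprite vertically.
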(event `self.ReceiveBeginPlay`
  (`KismetSystemLibrary.Delay` (`KismetMathLibrary.RandomFloatInRange` 0.1 0.3))
  (bind (_direction _alpha) (`Timeline|CloudAnim_Timeline` :!via `PlayFromStart`)
    (:`Update`
      (`SceneComponent.K2_SetRelativeLocation` (`self.PaperSprite`) (`KismetMathLibrary.MakeVector` 0.0 0.0 (`KismetMathLibrary.Lerp` 0.0 2.0 _alpha)) false false))))

(event `self.Hitbox.OnComponentBeginOverlap`
  (params (OverlappedComponent :type "PrimitiveComponent Object Reference") (OtherActor :type "Actor Object Reference") (OtherComp :type "PrimitiveComponent Object Reference") (OtherBodyIndex :type Integer) (bFromSweep :type Boolean) (SweepResult :type "HitResult Structure (by ref)"))
  (bind (_returnvalue_x _returnvalue_y _returnvalue_z) (`KismetMathLibrary.BreakVector` (* (`self.GetActorUpVector`) 1250.0)))
  (bind _as2dside_scroller_character (cast `/Game/2DSideScrollerBP/Blueprints/2DSideScrollerCharacter` OtherActor))
  (`Character.LaunchCharacter` _as2dside_scroller_character (`KismetMathLibrary.MakeVector` (`KismetMathLibrary.VSize` (* (`self.GetActorForwardVector` _as2dside_scroller_character) 15.0)) 0.0 _returnvalue_z) false true)
  (`GameplayStatics.PlaySound2D` "/Game/SFX/Environment/SC_CloudSound.SC_CloudSound" 1.0 1.0 0.0 null null)
  (`/Engine/EditorBlueprintResources/StandardMacros.DoOnce` false
    (:`Completed`
      (`PaperSpriteComponent.SetSprite` (`self.PaperSprite`) (`self.CloudSadFace`)))))

(fn `UserConstructionScript`
  (`PaperSpriteComponent.SetSprite` (`self.PaperSprite`) (`self.CloudHappyFace`)))