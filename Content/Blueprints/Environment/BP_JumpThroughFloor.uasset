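; BP_JumpThroughFloor is a Paper2D floor that, by its name, the player can jump through.
; The sprite starts with collision disabled.
; When an actor tagged Player enters the Box trigger, the sprite switches to query-only collision after a short delay.
; When the player leaves the Box, collision turns off again immediately, without cancelling any pending delay.
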(event `self.ReceiveBeginPlay`
  (`PrimitiveComponent.SetCollisionEnabled` (`self.PaperSprite`) "NoCollision"))

(event `self.Box.OnComponentBeginOverlap`
  (params (OverlappedComponent :type "PrimitiveComponent Object Reference") (OtherActor :type "Actor Object Reference") (OtherComp :type "PrimitiveComponent Object Reference") (OtherBodyIndex :type Integer) (bFromSweep :type Boolean) (SweepResult :type "HitResult Structure (by ref)"))
  (if (`self.ActorHasTag` OtherActor "Player")
    (`KismetSystemLibrary.Delay` 0.1)
    (`PrimitiveComponent.SetCollisionEnabled` (`self.PaperSprite`) "QueryOnly")))

(event `self.Box.OnComponentEndOverlap`
  (params (OverlappedComponent :type "PrimitiveComponent Object Reference") (OtherActor :type "Actor Object Reference") (OtherComp :type "PrimitiveComponent Object Reference") (OtherBodyIndex :type Integer))
  (if (`self.ActorHasTag` OtherActor "Player")
    (`PrimitiveComponent.SetCollisionEnabled` (`self.PaperSprite`) "NoCollision")))

(fn `UserConstructionScript`)