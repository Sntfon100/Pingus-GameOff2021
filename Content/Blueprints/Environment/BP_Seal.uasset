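; BP_Seal is a 2D seal hazard that leaps up when the player enters its trigger and kills the player through its hit box, each firing once.
; The Dive timeline drives the sprite's relative Z, scaled by JumpPower and paced by JumpPlayRate, with a sound on launch.
; If DiveDown is set, a DoN on the timeline's finish flips the sprite and reverses the dive, then restores its rotation.
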(event `self.ReceiveBeginPlay`
  (`TimelineComponent.SetPlayRate` (`self.Dive`) (`self.JumpPlayRate`)))

(event `self.Trigger.OnComponentBeginOverlap`
  (params (OverlappedComponent :type "PrimitiveComponent Object Reference") (OtherActor :type "Actor Object Reference") (OtherComp :type "PrimitiveComponent Object Reference") (OtherBodyIndex :type Integer) (bFromSweep :type Boolean) (SweepResult :type "HitResult Structure (by ref)"))
  (if (== OtherActor (`GameplayStatics.GetPlayerCharacter` 0))
    (`/Engine/EditorBlueprintResources/StandardMacros.DoOnce` false
      (:`Completed`
        (`self.DiveUp`)))))

(event `DiveUp`
  (bind _papersprite (`self.PaperSprite`))
  (bind (_relativelocation_x _relativelocation_y) (`KismetMathLibrary.BreakVector` (`SceneComponent.RelativeLocation` _papersprite)))
  (`GameplayStatics.PlaySound2D` "/Game/SFX/Pingus/SC_Seal.SC_Seal" 1.0 1.0 0.0 null null)
  (bind (_direction _newtrack_0) (`Timeline|Dive` :!via `PlayFromStart` :!label _label)
    (:`Update`
      (`SceneComponent.K2_SetRelativeLocation` _papersprite (`KismetMathLibrary.MakeVector` _relativelocation_x _relativelocation_y (* _newtrack_0 (`self.JumpPower`))) false false))
    (:`Finished`
      (if (`self.DiveDown?`)
        (bind _counter (`/Engine/EditorBlueprintResources/StandardMacros.Do N` 2)
          (:`Exit`
            (switch `int` _counter
              (:`1`
                (`self.DiveDown`))
              (:`2`
                (`SceneComponent.K2_SetRelativeRotation` :`self` (`self.PaperSprite`))))))))))

(event `StopMovement`
  (goto _label :!via `Stop`))

(event `DiveDown`
  (`SceneComponent.K2_SetRelativeRotation` (`self.PaperSprite`) (struct :`Pitch` 180.0) false false)
  (goto _label :!via `Reverse`))

(event `self.HitBox.OnComponentBeginOverlap`
  (params (OverlappedComponent :type "PrimitiveComponent Object Reference") (OtherActor :type "Actor Object Reference") (OtherComp :type "PrimitiveComponent Object Reference") (OtherBodyIndex :type Integer) (bFromSweep :type Boolean) (SweepResult :type "HitResult Structure (by ref)"))
  (bind _as2dside_scroller_character (cast `/Game/2DSideScrollerBP/Blueprints/2DSideScrollerCharacter` OtherActor))
  (`/Engine/EditorBlueprintResources/StandardMacros.DoOnce` false
    (:`Completed`
      (`/Game/2DSideScrollerBP/Blueprints/2DSideScrollerCharacter.OnPlayerDead` _as2dside_scroller_character true))))

(fn `UserConstructionScript`)