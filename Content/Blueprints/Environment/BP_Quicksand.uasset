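; Quicksand hazard that traps and sinks the 2D side-scroller character when it enters the hitbox.
; On overlap it flags the character as sinking, stops and slows it, and switches it to zero-gravity falling.
; A looping timer then offsets it vertically by SinkSpeed.
; On exit, it clears the timer and restores hard-coded walking settings only if the character overlaps no other quicksand.
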(event `self.Hitbox.OnComponentBeginOverlap`
  (params (OverlappedComponent :type "PrimitiveComponent Object Reference") (OtherActor :type "Actor Object Reference") (OtherComp :type "PrimitiveComponent Object Reference") (OtherBodyIndex :type Integer) (bFromSweep :type Boolean) (SweepResult :type "HitResult Structure (by ref)"))
  (bind _as2dside_scroller_character (cast `/Game/2DSideScrollerBP/Blueprints/2DSideScrollerCharacter` OtherActor))
  (set `/Game/2DSideScrollerBP/Blueprints/2DSideScrollerCharacter.isSinking?` true _as2dside_scroller_character)
  (bind _charactermovement (`Character.CharacterMovement` _as2dside_scroller_character))
  (`MovementComponent.StopMovementImmediately` _charactermovement)
  (set `CharacterMovementComponent.MaxWalkSpeed` 100.0 _charactermovement)
  (set `CharacterMovementComponent.GravityScale` 0.0 _charactermovement)
  (`CharacterMovementComponent.SetMovementMode` _charactermovement "MOVE_Falling" 0)
  (bind _returnvalue (`KismetSystemLibrary.K2_SetTimerDelegate` (delegate `SinkPlayer`) 0.1 true))
  (set `self.SinkTimer` _returnvalue))

(event `SinkPlayer`
  (`self.K2_AddActorWorldOffset` (stale `self.Hitbox.OnComponentBeginOverlap` _as2dside_scroller_character) (`KismetMathLibrary.MakeVector` 0.0 0.0 (`self.SinkSpeed`)) false false))

(event `self.Hitbox.OnComponentEndOverlap`
  (params (OverlappedComponent :type "PrimitiveComponent Object Reference") (OtherActor :type "Actor Object Reference") (OtherComp :type "PrimitiveComponent Object Reference") (OtherBodyIndex :type Integer))
  (bind _as2dside_scroller_character (cast `/Game/2DSideScrollerBP/Blueprints/2DSideScrollerCharacter` OtherActor))
  (if (not (> (`KismetArrayLibrary.Array_Length` (`self.GetOverlappingActors` _as2dside_scroller_character "BP_Quicksand_C")) 0))
    (`self.RestorePlayerMovement` (`Character.CharacterMovement` _as2dside_scroller_character) _as2dside_scroller_character)))

(event `RestorePlayerMovement`
  (params (MovementComp :type "CharacterMovementComponent Object Reference") (PlayerRef :type "/Game/2DSideScrollerBP/Blueprints/2DSideScrollerCharacter Object Reference"))
  (`KismetSystemLibrary.K2_ClearAndInvalidateTimerHandle` (`self.SinkTimer`))
  (set `CharacterMovementComponent.MaxWalkSpeed` 550.0 MovementComp)
  (set `CharacterMovementComponent.GravityScale` 2.0 MovementComp)
  (set `/Game/2DSideScrollerBP/Blueprints/2DSideScrollerCharacter.isSinking?` false PlayerRef)
  (`CharacterMovementComponent.SetMovementMode` MovementComp "MOVE_Walking" 0))

(fn `UserConstructionScript`)