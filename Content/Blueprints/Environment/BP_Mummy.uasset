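; BP_Mummy is a 2D side-scroller enemy that charges when it spots the player and kills it on contact.
; A Vision overlap with a Player-tagged actor plays an attack sound, switches to the run flipbook and enables Dash until a delay ends, then the mummy destroys itself.
; While dashing, Tick moves it unswept along the flipbook's negated forward vector, scaled by delta time.
; A HitBox overlap calls OnPlayerDead on the player character.
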(event `self.HitBox.OnComponentBeginOverlap`
  (params (OverlappedComponent :type "PrimitiveComponent Object Reference") (OtherActor :type "Actor Object Reference") (OtherComp :type "PrimitiveComponent Object Reference") (OtherBodyIndex :type Integer) (bFromSweep :type Boolean) (SweepResult :type "HitResult Structure (by ref)"))
  ;[1 1 1] Hitbox Overlap
  (bind _as2dside_scroller_character (cast `/Game/2DSideScrollerBP/Blueprints/2DSideScrollerCharacter` OtherActor))
  (`/Game/2DSideScrollerBP/Blueprints/2DSideScrollerCharacter.OnPlayerDead` _as2dside_scroller_character true))

(event `self.Vision.OnComponentBeginOverlap`
  (params (OverlappedComponent :type "PrimitiveComponent Object Reference") (OtherActor :type "Actor Object Reference") (OtherComp :type "PrimitiveComponent Object Reference") (OtherBodyIndex :type Integer) (bFromSweep :type Boolean) (SweepResult :type "HitResult Structure (by ref)"))
  ;[1 1 1] Vision Overlap
  (if (`self.ActorHasTag` OtherActor "Player")
    (set `self.Dash?` true)
    (`GameplayStatics.PlaySound2D` "/Game/SFX/Environment/SC_MummyAttack.SC_MummyAttack" 1.0 1.0 0.0 null null)
    (`PaperFlipbookComponent.SetFlipbook` (`self.PaperFlipbook`) "/Game/Sprites/Mummy/FB_Mummy_Run.FB_Mummy_Run")
    (`KismetSystemLibrary.Delay` (`self.DashDuration`))
    (set `self.Dash?` false)
    (`PaperFlipbookComponent.SetFlipbook` (`self.PaperFlipbook`) "/Game/Sprites/Mummy/FB_Mummy_Idle.FB_Mummy_Idle")
    (`self.K2_DestroyActor`)))

(event `self.ReceiveTick`
  (params (DeltaSeconds :type "Float (single-precision)"))
  (if (`self.Dash?`)
    (`self.LaunchForward` (`self.Launch Multiplier`))))

(fn `LaunchForward`
  (params (LaunchMultiplier :type "Float (double-precision)" :default 1000.0))
  (`self.K2_AddActorWorldOffset` (* (* (* (`KismetMathLibrary.GetForwardVector` (`SceneComponent.K2_GetComponentRotation` (`self.PaperFlipbook`))) -1.0) (`GameplayStatics.GetWorldDeltaSeconds`)) (`local.LaunchMultiplier`))))

(fn `UserConstructionScript`)